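; Smashable slime that slides along a set direction and is destroyed on overlap, adding scale-weighted points to the SNK game mode score.
; Its size follows Scale, and a death-animation actor spawns beneath it when smashed.
; Tick moves it by Speed and removes it beyond the X bounds.
; While the player is low, a slime approaching within a speed-sized distance reverses and flips to flee.
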(event `self.ReceiveBeginPlay`
  (bind _scale (`self.scale`))
  (`self.SetActorScale3D` (`KismetMathLibrary.MakeVector` _scale _scale _scale))
  (if (< (`self.speed`) 0.0)
    (`self.K2_AddActorLocalRotation` (struct :`Yaw` 180.0))))

(event `self.ReceiveActorBeginOverlap`
  (params (OtherActor :type "Actor Object Reference"))
  (bind _asgame_mode_snk (cast `/Game/Gameplay/GameModeSNK` (`GameplayStatics.GetGameMode`)))
  (set `/Game/Gameplay/GameModeSNK.Score` (+ (`/Game/Gameplay/GameModeSNK.Score` _asgame_mode_snk) (`KismetMathLibrary.FTrunc` (* (`self.value`) (`self.scale`)))) _asgame_mode_snk)
  (`|SpawnActorFromClass` "/Game/Smashable/Blueprint/animdeathslime.animdeathslime_C" (`KismetMathLibrary.MakeTransform` (- (`self.K2_GetActorLocation`) (0.0 0.0 15.0))) "Undefined" "OverrideRootScale" null null)
  (`self.K2_DestroyActor`))

(event `self.ReceiveTick`
  (params (DeltaSeconds :type "Float (single-precision)"))
  (bind _returnvalue_x (`KismetMathLibrary.BreakVector` (`self.K2_GetActorLocation`)))
  (bind _returnvalue_x_2 (`KismetMathLibrary.BreakVector` (`self.K2_GetActorLocation`)))
  (bind _returnvalue_x_3 (`KismetMathLibrary.BreakVector` (`self.K2_GetActorLocation`)))
  (bind _returnvalue_x_4 (`KismetMathLibrary.BreakVector` (`self.K2_GetActorLocation` (`GameplayStatics.GetPlayerCharacter` 0))))
  (bind (_returnvalue_x_5 _returnvalue_y _returnvalue_z) (`KismetMathLibrary.BreakVector` (`self.K2_GetActorLocation` (`GameplayStatics.GetPlayerCharacter` 0))))
  (bind _returnvalue_x_6 (`KismetMathLibrary.BreakVector` (`self.K2_GetActorLocation` (`GameplayStatics.GetPlayerCharacter` 0))))
  (`self.K2_SetActorLocation` (+ (* (`self.Direction`) (* DeltaSeconds (`self.speed`))) (`self.K2_GetActorLocation`)))
  (if (or (> _returnvalue_x_2 600.0) (< _returnvalue_x_2 -600.0))
    (`self.K2_DestroyActor`)
    (elif (< _returnvalue_z -40.0)
      (if (> (`self.speed`) 0.0)
        (if (and (> _returnvalue_x_3 (- _returnvalue_x_6 (`self.speed`))) (< _returnvalue_x_3 _returnvalue_x_6))
          (set `self.speed` (* -1 (`self.speed`)) :!label _label)
          (`self.K2_AddActorLocalRotation` (struct :`Yaw` 180.0)))
        (elif (and (< _returnvalue_x (- _returnvalue_x_4 (`self.speed`))) (> _returnvalue_x _returnvalue_x_4))
          (goto _label))))))

(fn `UserConstructionScript`)