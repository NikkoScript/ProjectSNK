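; PaperCharacterFoot is a player-controlled foot character that steps left or right along X and smashes downward on input.
; Smash stops movement, sets the speed and starts a Tick-driven descent via SetActorLocation to a fixed floor height, then Recharge raises it back above zero.
; BoolSmashing blocks move and smash input until both phases finish.
; Left and Right add movement input only on press, and the stored Target is never read here.
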(event `self.ReceiveTick`
  (params (DeltaSeconds :type "Float (single-precision)"))
  (bind (_returnvalue_x _returnvalue_y _returnvalue_z) (`KismetMathLibrary.BreakVector` (`self.K2_GetActorLocation`)))
  (bind (_returnvalue_x_2 _returnvalue_y_2 _returnvalue_z_2) (`KismetMathLibrary.BreakVector` (`self.K2_GetActorLocation`)))
  (if (`self.smash`)
    (`self.K2_SetActorLocation` (`KismetMathLibrary.MakeVector` _returnvalue_x _returnvalue_y (- _returnvalue_z (* DeltaSeconds (`self.speed`)))))
    (if (< _returnvalue_z -140.0)
      (set `self.recharge` true)
      (set `self.smash` false))
    (elif (`self.recharge`)
      (`self.K2_SetActorLocation` (`KismetMathLibrary.MakeVector` _returnvalue_x_2 _returnvalue_y_2 (- _returnvalue_z_2 (* (* DeltaSeconds (`self.speed`)) -1.0))))
      (if (< 0.0 _returnvalue_z_2)
        (set `self.recharge` false)
        (set `self.smash` false)))))

(event `InputAction|Left`
  (params (Key :type "Key Structure"))
  (:`Pressed`
    (if (`self.BoolSmashing`)
      (`self.AddMovementInput` (-1.0 0.0 0.0)))))

(event `InputAction|Right`
  (params (Key :type "Key Structure"))
  (:`Pressed`
    (if (`self.BoolSmashing`)
      (`self.AddMovementInput` (1.0 0.0 0.0)))))

(event `InputAction|Smash`
  (params (Key :type "Key Structure"))
  (bind (_returnvalue_x _returnvalue_y) (`KismetMathLibrary.BreakVector` (`self.K2_GetActorLocation`)))
  (:`Pressed`
    (if (`self.BoolSmashing`)
      (set `self.smash` true)
      (set `self.target` (`KismetMathLibrary.MakeVector` _returnvalue_x _returnvalue_y -140.0))
      (`MovementComponent.StopMovementImmediately` (`self.CharacterMovement`))
      (set `self.speed` 100.0))))

(fn `BoolSmashing`
  (returns (ReturnValue :type Boolean))
  (return (and (not (`self.smash`)) (not (`self.recharge`)))))

(fn `UserConstructionScript`)